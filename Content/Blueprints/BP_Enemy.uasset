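; Enemy pawn that chases the player once spotted and fires bullets that can damage them.
; PawnSensing sets a never-cleared sight flag and starts an AI move toward the player.
; Tick feeds a Delay that spawns bullets from the mesh's GunPoint socket periodically, regardless of sight.
; Health fills at BeginPlay; damage driving it below zero notifies BP_Player of the kill and destroys the enemy.
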(event `self.ReceiveBeginPlay`
  (`self.HealToFull`))

(event `self.ReceiveTick`
  (params (DeltaSeconds :type "Float (single-precision)"))
  (`KismetSystemLibrary.Delay` 1.5)
  (`self.ShootBullet`))

(event `self.PawnSensing.OnSeePawn`
  (params (Pawn :type "Pawn Object Reference"))
  (set `self.IsPlayerInSight` true)
  (`self.FollowPlayer`))

(event `FollowPlayer`
  (if (`self.IsPlayerInSight`)
    (`|AIMoveTo` self (0.0 0.0 0.0) (`GameplayStatics.GetPlayerCharacter` 0) 500.0 true)))

(event `OnDeath`
  (bind _asbp_player (cast `/Game/Blueprints/BP_Player` (`GameplayStatics.GetPlayerCharacter` 0)))
  (`/Game/Blueprints/BP_Player.OnEnemyKilled` _asbp_player self)
  (`self.K2_DestroyActor`))

(fn `HealToFull`
  (set `self.CurrentHealth` (`self.MaxHealth`)))

(fn `ShootBullet`
  (returns (SpawnedBullet :type "/Game/Blueprints/BP_Bullet Object Reference"))
  (bind _returnvalue (`|SpawnActorFromClass` "/Game/Blueprints/BP_Bullet.BP_Bullet_C" (`SceneComponent.GetSocketTransform` (`self.SM_Enemy`) "GunPoint" "RTS_World") "Undefined" "MultiplyWithRoot" null null))
  (set `/Game/Blueprints/BP_Bullet.WillDamagePlayer` true _returnvalue)
  (return _returnvalue))

(fn `TakeDamage`
  (params (Damage :type Integer))
  (bind _output_get (set `self.CurrentHealth` (- (`self.CurrentHealth`) Damage)))
  ; Handle <0 hp
  (if (< _output_get 0)
    (set `self.CurrentHealth` 0)
    (`self.OnDeath`)
    (else
      ; Handle >Max hp
      (if (> 0 (`self.MaxHealth`))
        (set `self.CurrentHealth` (`self.MaxHealth`))))))

(fn `UserConstructionScript`)